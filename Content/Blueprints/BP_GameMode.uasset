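; Game mode that configures a match for the Endless or Race game type and tracks player speed for display.
; SetupMode picks the HUD and pawn classes, shows the widget, then initializes the player controller at the player start.
; Both types share the Endless HUD, and the controller always receives Endless as its game type.
; Each tick, UpdateHUD converts the controller's speed reference through VelocityToMS into the speed text.
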(event `self.ReceiveTick`
  (params (DeltaSeconds :type "Float (single-precision)"))
  ;[1 1 1] Update
  (`self.UpdateHUD`))

(fn `SetupMode`
  (params (GameType :type "/Game/Data/ENUM_GameType Enum" :default "NewEnumerator0"))
  (locals (HUDUsed :type "UserWidget Class Reference") (PlayerUsed :type "/Game/Blueprints/Player/BP_Player Class Reference"))
  ;[1 1 1] Set classes based on game type
  (switch `/Game/Data/ENUM_GameType` GameType
    (:`NewEnumerator0`
      (set `local.HUDUsed` "/Game/HUD/BP_HUD_Endless.BP_HUD_Endless_C")
      (set `local.PlayerUsed` "/Game/Blueprints/Player/BP_Player_Endless.BP_Player_Endless_C"))
    (:`NewEnumerator1`
      (set `local.HUDUsed` "/Game/HUD/BP_HUD_Endless.BP_HUD_Endless_C")
      (set `local.PlayerUsed` "/Game/Blueprints/Player/BP_Player_Race.BP_Player_Race_C")))
  ;[1 1 1] HUD setup
  (bind _returnvalue (`|CreateWidget` (`local.HUDUsed`)))
  (bind _output_get (set `self.HUDOReference` _returnvalue))
  (`UserWidget.AddToViewport` _output_get 0)
  ;[1 1 1] Player controller setup
  (set `self.DefaultPawnClass` (`local.PlayerUsed`))
  (bind _asbp_player_controller (cast `/Game/Blueprints/Player/BP_PlayerController` (`GameplayStatics.GetPlayerController` 0)))
  (set `self.PlayerControllerOReference` _asbp_player_controller)
  (`/Game/Blueprints/Player/BP_PlayerController.InitializeController` (`self.PlayerControllerOReference`) (`self.K2_GetActorLocation` (`self.K2_FindPlayerStart` null)) (`local.PlayerUsed`) self "NewEnumerator0"))

(fn `UpdateHUD`
  (set `self.PlayerSpeedText` (`/Game/Blueprints/BP_Macros.VelocityToM/S` (`/Game/Blueprints/Player/BP_PlayerController.PlayerSpeedRef` (`self.PlayerControllerOReference`)))))

(fn `UserConstructionScript`)