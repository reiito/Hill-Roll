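; BP_Tracker is an actor that applies level settings to the player controller and triggers the player spawn at BeginPlay.
; It first caches cast references to BP_PlayerController and BP_GameMode, though the game mode reference is not used further here.
; It then copies its reposition cap, camera angle and distance, and respawn delay variables into the controller before calling SpawnPlayer.
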(event `self.ReceiveBeginPlay`
  ;[1 1 1] Begin play
  (`self.SetupReferences`)
  (`self.ApplyLevelParameters`)
  (`/Game/Blueprints/Player/BP_PlayerController.SpawnPlayer` (`self.PlayerControllerOReference`)))

(fn `ApplyLevelParameters`
  ;[1 1 1] Load modified parameters into level
  (set `/Game/Blueprints/Player/BP_PlayerController.LevelRepositionCap` (`self.RepositionCap`) (`self.PlayerControllerOReference`))
  (set `/Game/Blueprints/Player/BP_PlayerController.LevelRotationY` (`self.CameraAngle`) (`self.PlayerControllerOReference`))
  (set `/Game/Blueprints/Player/BP_PlayerController.PlayerRespawnTime` (`self.RespawnDelay`) (`self.PlayerControllerOReference`))
  (set `/Game/Blueprints/Player/BP_PlayerController.PlayerCameraDistance` (`self.CameraDistance`) (`self.PlayerControllerOReference`)))

(fn `SetupReferences`
  (locals (CurrentPlayer :type "Object Object Reference"))
  (bind _asbp_player_controller (cast `/Game/Blueprints/Player/BP_PlayerController` (`GameplayStatics.GetPlayerController` 0)))
  (set `self.PlayerControllerOReference` _asbp_player_controller)
  (bind _asbp_game_mode (cast `/Game/Blueprints/BP_GameMode` (`GameplayStatics.GetGameMode`)))
  (set `self.GameModeOReference` _asbp_game_mode))

(fn `UserConstructionScript`)