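; Pickup actor that animates its Pickup component with a spin and a vertical bob, with no collection logic in the event graph.
; On BeginPlay, it caches the start location, derives the end point from a Z offset, and sets both timelines' play rates from speed variables.
; One timeline lerps world rotation, while the other lerps location and ping-pongs by re-entering a FlipFlop on Finished to alternate Play and Reverse.
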(event `PlayRotationAnimation`
  ;[1 1 1] Animations
  (bind (_direction _rotationalpha) (`Timeline|RotationAnimation`)
    (:`Update`
      (`SceneComponent.K2_SetWorldRotation` (`self.Pickup`) (`KismetMathLibrary.RLerp` (struct) (struct :`Yaw` 360.0) _rotationalpha) false false))))

(event `self.ReceiveBeginPlay`
  ;[1 1 1] Startup
  (`self.SetupAnimation`)
  (`self.PlayRotationAnimation`)
  (`self.PlayMovementAnimation`))

(event `PlayMovementAnimation`
  ;[1 1 1] Animations
  (`/Engine/EditorBlueprintResources/StandardMacros.FlipFlop`
    (:`A`
      (bind (_direction _movementalpha) (`Timeline|Movement Animation` :!label _label)
        (:`Update`
          (`SceneComponent.K2_SetWorldLocation` (`self.Pickup`) (`KismetMathLibrary.VLerp` (`self.StartLocation`) (`self.EndLocation`) _movementalpha) false false))
        (:`Finished`
          (`self.PlayMovementAnimation`))))
    (:`B`
      (goto _label :!via `Reverse`))))

(fn `SetupAnimation`
  ;[1 1 1] Determine start and end points for movement animation/ping pong points
  (bind _output_get (set `self.StartLocation` (`SceneComponent.K2_GetComponentLocation` (`self.Pickup`))))
  (set `self.EndLocation` (+ _output_get (`KismetMathLibrary.MakeVector` 0.0 0.0 (`self.MovementAnimationZShift`))))
  ;[1 1 1] Modify how fast animations run
  (`TimelineComponent.SetPlayRate` (`self.RotationAnimation`) (`self.RotationAnimationSpeed`))
  (`TimelineComponent.SetPlayRate` (`self.Movement Animation`) (`self.MovementAnimationSpeed`)))

(fn `UserConstructionScript`)