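; Sloped track tile for the endless mode that randomly builds its content in the Construction Script, then pitches itself by TileRot.
; It adds instanced fences, flora, trees and clouds, then spawns obstacles and chance-based money pickups across five lanes, shifting pickups that match a recorded obstacle X.
; AttachPoint exposes a transform for attachment.
; When the player hits EndTrigger, BP_GameMode_Endless adds another tile, possibly a split, and this one destroys itself after a delay.
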(event `self.EndTrigger.OnComponentBeginOverlap`
  (params (OverlappedComponent :type "PrimitiveComponent Object Reference") (OtherActor :type "Actor Object Reference") (OtherComp :type "PrimitiveComponent Object Reference") (OtherBodyIndex :type Integer) (bFromSweep :type Boolean) (SweepResult :type "HitResult Structure (by ref)"))
  (cast `/Game/Blueprints/Player/BP_Player` OtherActor)
  (bind _asbp_game_mode_endless (cast `/Game/Blueprints/BP_GameMode_Endless` (`GameplayStatics.GetGameMode`)))
  (`/Game/Blueprints/BP_GameMode_Endless.AddRandomTile` _asbp_game_mode_endless (`KismetMathLibrary.RandomBoolWithWeight` (`self.SplitSpawnWeight`)))
  (`KismetSystemLibrary.Delay` 5.0)
  (`self.K2_DestroyActor`))

(fn `ConstructFences`
  (params (NumSegments :type Integer))
  (locals (SegmentShift :type "Float (double-precision)") (NumSeg :type Integer) (CurrentSegmentPos :type "Float (double-precision)" :default -250.0) (GroundDimensions :type "Vector Structure") (FenceLocation :type "Vector Structure") (GroundLength :type "Float (double-precision)" :default 1200.0))
  (bind (_grounddimensions_x _grounddimensions_y _grounddimensions_z) (`KismetMathLibrary.BreakVector` (`local.GroundDimensions`)))
  (bind (_fencelocation_x _fencelocation_y _fencelocation_z) (`KismetMathLibrary.BreakVector` (`local.FenceLocation`)))
  (bind (_grounddimensions_x_2 _grounddimensions_y_2) (`KismetMathLibrary.BreakVector` (`local.GroundDimensions`)))
  (bind (_returnvalue_x _returnvalue_y _returnvalue_z) (`KismetMathLibrary.BreakVector` (`SceneComponent.K2_GetComponentLocation` (`self.Ground`))))
  (bind (_returnvalue_x_2 _returnvalue_y_2) (`KismetMathLibrary.BreakVector2D` (+ (`KismetMathLibrary.MakeVector2D` _returnvalue_y _returnvalue_z) (`KismetMathLibrary.MakeVector2D` _grounddimensions_y _grounddimensions_z))))
  (`|ExecutionSequence`
    (:`then_0`
      ;[1 1 1] [New] - Forgo calculating number of segments required, manually type in for tiles instead.
      (set `local.GroundDimensions` (`.BoxExtent` (`KismetSystemLibrary.GetComponentBounds` (`self.Ground`))))
      (set `local.SegmentShift` (* 2 (.x (`.BoxExtent` (`KismetSystemLibrary.GetComponentBounds` (`self.FenceReference`))))))
      (set `local.FenceLocation` (`KismetMathLibrary.MakeVector` (- _returnvalue_x _grounddimensions_x) _returnvalue_x_2 _returnvalue_y_2))
      (set `local.NumSeg` NumSegments)
      ;[1 1 1] Generate segments for fences
      (`self.CreateFenceSegments` (`self.RightFence`) (`local.FenceLocation`) (`local.SegmentShift`) (`local.NumSeg`))
      (`self.CreateFenceSegments` (`self.LeftFence`) (`KismetMathLibrary.MakeVector` _fencelocation_x (- _fencelocation_y (* 2 _grounddimensions_y_2)) _fencelocation_z) (`local.SegmentShift`) (`local.NumSeg`))
      ;[1 1 1] Remove reference, no longer needed
      (`ActorComponent.K2_DestroyComponent` (`self.FenceReference`)))
    (:`then_1`
      ;[1 1 1] Determine whether outer grass area should be shown
      (if (not (`self.ShowOuterGrass`))
        (`SceneComponent.ToggleVisibility` (`self.OuterGrassRight`) false)
        (`SceneComponent.ToggleVisibility` (`self.OuterGrassLeft`) false)))))

(fn `CreateFenceSegments`
  (params (Fence :type "InstancedStaticMeshComponent Object Reference") (Position :type "Vector Structure") (SegmentShift :type "Float (double-precision)") (NumSegments :type Integer))
  (locals (CurrentSegmentPos :type "Float (double-precision)"))
  ;[1 1 1] Position fence on matching side of ground
  (`SceneComponent.K2_SetWorldLocation` Fence Position false false)
  ;[1 1 1] Loop and create segments until end of ground end
  (for _ (range (`local.NumSegments`))
    (`InstancedStaticMeshComponent.AddInstance` (`local.Fence`) (`KismetMathLibrary.MakeTransform` (`KismetMathLibrary.MakeVector` (`local.CurrentSegmentPos`))))
    (set `local.CurrentSegmentPos` (+ (`local.CurrentSegmentPos`) (`local.SegmentShift`)))))

(fn `CreateLanes`
  (set `self.LaneArray` (`|MakeArray` (`self.MiddleLane`) (`self.LeftLane1`) (`self.LeftLane2`) (`self.RightLane1`) (`self.RightLane2`))))

(fn `GetAttachTransform`
  (returns (Transform :type "Transform Structure"))
  (return (`SceneComponent.K2_GetComponentToWorld` (`self.AttachPoint`))))

(fn `SetupObstacleSpawnPoints`)

(fn `SpawnClouds`
  (params (MaxCLouds :type Integer))
  (locals (MinClouds :type Integer :default 2))
  (for _ (range (`KismetMathLibrary.RandomIntegerInRange` (`local.MinClouds`) MaxCLouds))
    (bind _location (`self.SpawnRandomLocation` (`self.CloudsSpawn`)))
    (bind _returnvalue (`AddComponent|NODE_AddStaticMeshComponent-4` :`RelativeTransform` _location))
    (`PrimitiveComponent.SetRenderCustomDepth` _returnvalue true)
    (`StaticMeshComponent.SetStaticMesh` _returnvalue (`/Game/Blueprints/BP_Macros.SelectRandomFromArray` (`self.Clouds`)))
    (`PrimitiveComponent.SetCollisionEnabled` _returnvalue "NoCollision")))

(fn `SpawnDecor`
  (`self.ConstructFences` (`self.NumSegments`))
  (`self.SpawnFlora`)
  (`self.SpawnOuterArea`))

(fn `SpawnFlora`
  (bind _tilerot (`self.TileRot`))
  (bind _florasize (`self.FloraSize`))
  (for _ (range (+ (`self.NumFlora`) 1))
    (bind _location (`self.SpawnRandomLocation` (`self.FloraSpawn`)))
    (`AddComponent|NODE_AddChildActorComponent-4` :`RelativeTransform` (`KismetMathLibrary.MakeTransform` (.location _location) (`KismetMathLibrary.MakeRotator` 0.0 (`KismetMathLibrary.RandomFloatInRange` (* -1 _tilerot) _tilerot) (`KismetMathLibrary.RandomFloatInRange` 0.0 360.0)) (`KismetMathLibrary.MakeVector` _florasize _florasize _florasize)))))

(fn `SpawnInSequence`
  (params (`Bounding box` :type "BoxComponent Object Reference") (Count :type Integer) (Actor :type "Actor Class Reference"))
  (locals (Spacing :type "Float (double-precision)") (Position :type "Vector Structure"))
  (bind (_relativelocation_x _relativelocation_y _relativelocation_z) (`KismetMathLibrary.BreakVector` (`SceneComponent.RelativeLocation` `Bounding box`)))
  (bind (_position_x _position_y _position_z) (`KismetMathLibrary.BreakVector` (`local.Position`)))
  (bind _returnvalue (- (`local.Count`) 1))
  (set `local.Position` (`KismetMathLibrary.MakeVector` 0.0 _relativelocation_y _relativelocation_z))
  (set `local.Spacing` (/ (* _relativelocation_x 2.0) (`KismetMathLibrary.Conv_IntToDouble` _returnvalue)))
  (for _ (range (+ _returnvalue 1))
    (bind _returnvalue_2 (`AddComponent|NODE_AddChildActorComponent-13` :`RelativeTransform` (`KismetMathLibrary.Conv_VectorToTransform` (`local.Position`))))
    (`ChildActorComponent.SetChildActorClass` _returnvalue_2 (`local.Actor`))
    (set `local.Position` (`KismetMathLibrary.MakeVector` (+ (`local.Spacing`) _position_x) _position_y _position_z))))

(fn `SpawnInteractables`
  (`self.SpawnObstacles`)
  (`self.SpawnPickups`))

(fn `SpawnObstacles`
  ;[1 1 1] Set size of spawn points to match total number of obstacles
  (`KismetArrayLibrary.Array_Resize` (`self.ObstacleSpawnPoints`) (* (`self.ObstaclesPerLane`) (`KismetArrayLibrary.Array_Length` (`self.LaneArray`))))
  (for (_array_element _array_index) (`self.LaneArray`)
    ;[1 1 1] Create random spawn point and spawn a random obstacle
    (bind _location (`self.SpawnRandomLocation` _array_element))
    (`KismetArrayLibrary.Array_Set` (`self.ObstacleSpawnPoints`) _array_index (`KismetMathLibrary.Round` (.x (.location _location))))
    (bind _returnvalue (`AddComponent|NODE_AddChildActorComponent-8` :`RelativeTransform` _location))
    (`ChildActorComponent.SetChildActorClass` _returnvalue (`/Game/Blueprints/BP_Macros.SelectRandomFromArray` (`self.Obstacles`)))))

(fn `SpawnOuterArea`
  (locals (MaxTreeSpawns :type Integer :default 12) (MinTreeSpawns :type Integer :default 6) (MinCloudSpawns :type Integer :default 0) (MaxCloudSpawns :type Integer :default 6))
  (bind _returnvalue (`KismetMathLibrary.RandomIntegerInRange` (`local.MinTreeSpawns`) (`local.MaxTreeSpawns`)))
  ;[1 1 1] Populate sides with trees
  (`self.SpawnInSequence` (`self.OuterTreesRight`) _returnvalue "/Game/Blueprints/Level/Obstacles/BP_Tree.BP_Tree_C")
  (`self.SpawnInSequence` (`self.OuterTreesLeft`) _returnvalue "/Game/Blueprints/Level/Obstacles/BP_Tree.BP_Tree_C")
  ;[1 1 1] Fill sky with clouds
  (for _ (range (`KismetMathLibrary.RandomIntegerInRange` (`local.MinCloudSpawns`) (`local.MaxCloudSpawns`)))
    (bind _location (`self.SpawnRandomLocation` (`self.CloudsSpawn`)))
    (bind _returnvalue_2 (`AddComponent|NODE_AddStaticMeshComponent-3` :`RelativeTransform` _location))
    (`PrimitiveComponent.SetRenderCustomDepth` _returnvalue_2 true)
    (`StaticMeshComponent.SetStaticMesh` _returnvalue_2 (`/Game/Blueprints/BP_Macros.SelectRandomFromArray` (`self.Clouds`)))
    (`PrimitiveComponent.SetCollisionEnabled` _returnvalue_2 "NoCollision")))

(fn `SpawnPickups`
  (locals (SpawnPoint :type "Transform Structure"))
  (for _array_element (`self.LaneArray`)
    ;[1 1 1] Random chance to spawn pickup
    (if (`KismetMathLibrary.RandomBoolWithWeight` (`self.PickupSpawnChance`))
      ;[1 1 1] Generate random location, if matches location of obstacle, add offset to location
      (bind _location (`self.SpawnRandomLocation` _array_element))
      (bind _output_get (set `local.SpawnPoint` _location))
      (if (`KismetArrayLibrary.Array_Contains` (`self.ObstacleSpawnPoints`) (`KismetMathLibrary.Round` (.x (.location _output_get))))
        (set `local.SpawnPoint` (`KismetMathLibrary.MakeTransform` (`KismetMathLibrary.MakeVector` (+ (`self.PickupSpawnOffset`) (.x (.location _output_get))) (.y (.location _output_get)) (.z (.location _output_get))) (.rotation _output_get) (.scale _output_get))))
      (bind _returnvalue (`AddComponent|NODE_AddChildActorComponent-14` :`RelativeTransform` (`local.SpawnPoint`)))
      (`ChildActorComponent.SetChildActorClass` _returnvalue "/Game/Blueprints/Level/Pickups/BP_Pickup_Money.BP_Pickup_Money_C") ; TODO: Random powerup or money, currently money only
    )))

(fn `SpawnRandomLocation`
  (params (BoundingBox :type "BoxComponent Object Reference"))
  (returns (Location :type "Transform Structure"))
  (return (`KismetMathLibrary.Conv_VectorToTransform` (`KismetMathLibrary.RandomPointInBoundingBox` (`SceneComponent.RelativeLocation` BoundingBox) (`BoxComponent.BoxExtent` BoundingBox)))))

(fn `SpawnTrees`
  (params (MaxTrees :type Integer))
  (locals (MinTrees :type Integer :default 5))
  (bind _returnvalue (`KismetMathLibrary.RandomIntegerInRange` (`local.MinTrees`) MaxTrees))
  ;[1 1 1] Populate sides with trees
  (`self.SpawnInSequence` (`self.OuterTreesRight`) _returnvalue "/Game/Blueprints/Level/Obstacles/BP_Tree.BP_Tree_C")
  (`self.SpawnInSequence` (`self.OuterTreesLeft`) _returnvalue "/Game/Blueprints/Level/Obstacles/BP_Tree.BP_Tree_C"))

(fn `UserConstructionScript`
  (`self.CreateLanes`)
  (`self.SpawnDecor`)
  (`self.SpawnInteractables`)
  (`self.K2_SetActorRotation` (`KismetMathLibrary.MakeRotator` 0.0 (`self.TileRot`))))