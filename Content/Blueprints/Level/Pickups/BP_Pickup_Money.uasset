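; Money pickup Blueprint that appears as a small, medium or large crystal, each worth a different amount.
; On BeginPlay it runs the parent logic, then calls SetValue with randomization on, replacing the passed size with a pick from RandomValues.
; SetValue assigns the matching mesh and value, then stores the chosen size as its Type.
; UpdateMoneyEarned is an empty stub here.
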(event `self.ReceiveBeginPlay`
  (`parent.ReceiveBeginPlay`)
  (`self.SetValue` "NewEnumerator0" true))

(fn `SetValue`
  (params (SetValue :type "/Game/Data/ENUM_MoneyValues Enum" :default "NewEnumerator0") (Random :type Boolean))
  (locals (PickupMesh :type "StaticMesh Object Reference") (ChosenType :type "/Game/Data/ENUM_MoneyValues Enum"))
  (set `local.ChosenType` SetValue)
  (`|ExecutionSequence`
    (:`then_0`
      ;[1 1 1] If randomize on, overwrite value with random one
      (if Random
        (set `local.ChosenType` (`/Game/Blueprints/BP_Macros.SelectRandomFromArray` (`self.RandomValues`)))))
    (:`then_1`
      ;[1 1 1] Display appropriate mesh and assign value depending on type
      (switch `/Game/Data/ENUM_MoneyValues` (`local.ChosenType`)
        (:`NewEnumerator0`
          (set `local.PickupMesh` "/Game/Models/Level/Crystal.Crystal")
          (set `self.Value` 5))
        (:`NewEnumerator1`
          (set `local.PickupMesh` "/Game/Models/Level/CrystalMedium.CrystalMedium")
          (set `self.Value` 25))
        (:`NewEnumerator2`
          (set `local.PickupMesh` "/Game/Models/Level/CrystalLarge.CrystalLarge")
          (set `self.Value` 100)))
      (`StaticMeshComponent.SetStaticMesh` (`self.Pickup`) (`local.PickupMesh`)))
    (:`then_2`
      ;[1 1 1] Update money type
      (set `self.Type` (`local.ChosenType`)))))

(fn `UpdateMoneyEarned`)

(fn `UserConstructionScript`
  (`parent.UserConstructionScript`))