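; Slope tile Blueprint that lays out a grid of fail spikes as child actors at construction time.
; After the parent construction script runs, SpawnSpikes starts at the relative location of Start0 and fills rows along X, stepping across each on Y.
; Row and column counts, Spacing0 and a uniform Scale shape the grid, while height stays fixed at the start point's Z.
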(fn `SpawnSpikes`
  (locals (SpikeShiftUp :type "Float (double-precision)") (SpikeShiftAcross :type "Float (double-precision)") (SpikeZPos :type "Float (double-precision)"))
  (bind (_spacing_0_x _spacing_0_y) (`KismetMathLibrary.BreakVector2D` (`self.Spacing_0`)))
  (bind _spacing_0_x_2 (`KismetMathLibrary.BreakVector2D` (`self.Spacing_0`)))
  (bind _scale (`self.Scale`))
  (bind (_relativelocation_x _relativelocation_y) (`KismetMathLibrary.BreakVector` (`SceneComponent.RelativeLocation` (`self.Start_0`))))
  (bind (_relativelocation_x_2 _relativelocation_y_2 _relativelocation_z) (`KismetMathLibrary.BreakVector` (`SceneComponent.RelativeLocation` (`self.Start_0`))))
  ;[1 1 1] Set starting positions
  (set `local.SpikeShiftUp` _relativelocation_x_2)
  (set `local.SpikeShiftAcross` _relativelocation_y_2)
  (set `local.SpikeZPos` _relativelocation_z)
  ;[1 1 1] Create Rows (Bottom up)
  (for _ (range (`self.NumRows`))
    ;[1 1 1] Reset shift across for each new row. First spike's across position matches start
    (set `local.SpikeShiftAcross` _relativelocation_y)
    ;[1 1 1] Populate row
    (for _ (range (`self.NumCols`))
      (`AddComponent|NODE_AddChildActorComponent-4` :`RelativeTransform` (`KismetMathLibrary.MakeTransform` (`KismetMathLibrary.MakeVector` (`local.SpikeShiftUp`) (`local.SpikeShiftAcross`) (`local.SpikeZPos`)) (struct) (`KismetMathLibrary.MakeVector` _scale _scale _scale)))
      ;[1 1 1] Update spacing between spikes
      (set `local.SpikeShiftAcross` (+ (`local.SpikeShiftAcross`) _spacing_0_y)))
    ;[1 1 1] Move up to next row
    (set `local.SpikeShiftUp` (+ (`local.SpikeShiftUp`) _spacing_0_x_2))))

(fn `UserConstructionScript`
  (`parent.UserConstructionScript`)
  (`self.SpawnSpikes`))