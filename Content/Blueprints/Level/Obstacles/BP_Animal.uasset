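; Animal obstacle that paces sideways along world Y, with randomized speed, turn rate and starting direction set on activation at BeginPlay.
; Fence overlaps pause it for a random wait, then a FlipFlop-driven rotation timeline turns it, with movement resuming inverted on forward completion.
; Hitting obstacles, or optionally the player, stops the jump timeline and enables model physics.
; AdjustParameters overrides tuning; a self-looping Jump event exists but is not started here, and head-bobbing is disconnected.
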(event `StopJumping`
  (bind (_returnvalue_x _returnvalue_y) (`KismetMathLibrary.BreakVector` (`self.K2_GetActorLocation`)))
  ;[1 1 1] Make animal jump up and down, stop when its turning
  (bind (_direction _jumpalpha) (`Timeline|JumpTimeline` :!via `Stop` :!label _label)
    (:`Update`
      (`self.K2_SetActorLocation` (`KismetMathLibrary.MakeVector` _returnvalue_x _returnvalue_y (`KismetMathLibrary.Lerp` (`self.GroundLocation`) (`self.JumpPeak`) _jumpalpha))))
    (:`Finished`
      (`self.Jump`))))

(event `Jump`
  ;[1 1 1] Make animal jump up and down, stop when its turning
  (`/Engine/EditorBlueprintResources/StandardMacros.FlipFlop`
    (:`A`
      (goto _label))
    (:`B`
      (goto _label :!via `ReverseFromEnd`))))

(event `self.ReceiveTick`
  (params (DeltaSeconds :type "Float (single-precision)"))
  ;[1 1 1] Movement
  (`self.MoveAnimal`))

(event `self.ReceiveBeginPlay`
  ;[1 1 1] Leave blank at end, activate when ready
  (`self.Activate`))

(event `MoveAnimal`
  (bind _animal (`self.Animal`))
  (bind (_returnvalue_x _returnvalue_y _returnvalue_z) (`KismetMathLibrary.BreakVector` (`SceneComponent.K2_GetComponentLocation` _animal)))
  ;[1 1 1] Movement
  ;;[1 1 1] Left->Right / Right->Left
  (if (`self.Moving`)
    (`SceneComponent.K2_SetWorldLocation` _animal (`KismetMathLibrary.MakeVector` _returnvalue_x (+ _returnvalue_y (* (`GameplayStatics.GetWorldDeltaSeconds`) (* (`self.MaxSpeed`) (`self.SpeedMultiplier`)))) _returnvalue_z) false false)))

(event `Change Direction`
  (bind _facingdirection (`self.FacingDirection`))
  ;[1 1 1] Movement
  ;;[1 1 1] Direction change behaviour = Wait a couple of seconds then animate to turn around, then continue moving
  (set `self.Moving` false)
  (`KismetSystemLibrary.Delay` (`KismetMathLibrary.RandomFloatInRange` 1.0 (`self.MaxWaitTime`)))
  (`/Engine/EditorBlueprintResources/StandardMacros.FlipFlop`
    (:`A`
      (bind (_direction _rotation) (`Timeline|RotationTimeline` :!via `PlayFromStart` :!label _label_2)
        (:`Update`
          (`SceneComponent.K2_SetWorldRotation` (`self.Animal`) (`KismetMathLibrary.RLerp` _facingdirection (* _facingdirection -1) _rotation) false false))
        (:`Finished`
          ;;;[1 1 1] Enable moving again and invert speed
          (set `self.Moving` true)
          (set `self.MaxSpeed` (* -1 (`self.MaxSpeed`))))))
    (:`B`
      (goto _label_2 :!via `ReverseFromEnd`))))

(event `self.GeneralCollision.OnComponentBeginOverlap`
  (params (OverlappedComponent :type "PrimitiveComponent Object Reference") (OtherActor :type "Actor Object Reference") (OtherComp :type "PrimitiveComponent Object Reference") (OtherBodyIndex :type Integer) (bFromSweep :type Boolean) (SweepResult :type "HitResult Structure (by ref)"))
  ;[1 1 1] Check for collision with obstacles and player, fence to change direction
  (bind _tag (`/Game/Blueprints/BP_Macros.GetComponentTag` 0 OtherComp)
    (:`__`
      (switch `string` _tag
        (:`Obstacle`
          (`self.Collide`))
        (:`Player`
          (if (`self.ReactToPlayer`)
            (`self.Collide`)))))))

(event `self.FenceCollision.OnComponentBeginOverlap`
  (params (OverlappedComponent :type "PrimitiveComponent Object Reference") (OtherActor :type "Actor Object Reference") (OtherComp :type "PrimitiveComponent Object Reference") (OtherBodyIndex :type Integer) (bFromSweep :type Boolean) (SweepResult :type "HitResult Structure (by ref)"))
  ;[1 1 1] Check for collision with obstacles and player, fence to change direction
  (bind _tag (`/Game/Blueprints/BP_Macros.GetComponentTag` 0 OtherComp)
    (:`__`
      (if (`KismetStringLibrary.EqualEqual_StrStr` _tag "Fence")
        (`self.Change Direction`)))))

(fn `Activate`
  ;[1 1 1] Initialize then start animal behaviour
  (`self.Initialize`)
  (set `self.Moving` true))

(fn `AdjustParameters`
  (params (DurationTurn :type "Float (double-precision)") (DurationJump :type "Float (double-precision)") (HeightJump :type "Float (double-precision)") (RotationSideToSide :type "Float (double-precision)") (SizeScaling :type "Vector Structure") (ReactOnPlayerContact :type Boolean) (PlayerReactsTo :type Boolean) (AnimalCanJump :type Boolean))
  (bind _durationjump (`local.DurationJump`))
  (bind _heightjump (`local.HeightJump`))
  (bind _rotationsidetoside (`local.RotationSideToSide`))
  (bind _durationturn (`local.DurationTurn`))
  (bind (_sizescaling_x _sizescaling_y _sizescaling_z) (`KismetMathLibrary.BreakVector` (`local.SizeScaling`)))
  ;[1 1 1] Assign point a and b and bool regardless of value
  (set `self.ReactToPlayer` (`local.ReactOnPlayerContact`))
  (set `self.PlayerReactWith` (`local.PlayerReactsTo`))
  (set `self.JumpEnabled` (`local.AnimalCanJump`))
  (`|ExecutionSequence`
    (:`then_0`
      ;[1 1 1] Replace when values assigned not 0 or blank
      ;;[1 1 1] Assign only when values not left blank
      (if (> _durationturn 0.0)
        (set `self.TurnMaxDuration` _durationturn)))
    (:`then_1`
      (if (> _durationjump 0.0)
        (set `self.JumpDuration` _durationjump)))
    (:`then_2`
      (if (> _heightjump 0.0)
        (set `self.JumpHeight` _heightjump)))
    (:`then_3`
      (if (> _rotationsidetoside 0.0)
        (set `self.SideToSideRot` _rotationsidetoside)))
    (:`then_4`
      ;;[1 1 1] Assign when all scaling dimensions > 0
      (if (and (> _sizescaling_x 0.0) (> _sizescaling_y 0.0) (> _sizescaling_z 0.0))
        (set `self.Size` (`local.SizeScaling`))))))

(fn `Collide`
  ;[1 1 1] Stop all lerping movement, simulate physics
  (`self.StopJumping`)
  (`PrimitiveComponent.SetSimulatePhysics` (`self.Model`) true))

(fn `Initialize`
  (`self.RandomizeSettings`)
  ;[1 1 1] When animal is set to enable player reaction, give them the obstacle tag
  (if (`self.PlayerReactWith`)
    (set `ActorComponent.ComponentTags` (`|MakeArray` "Obstacle" "Animal" :!type "Name") (`self.Model`))))

(fn `RandomizeSettings`
  (locals (Left :type "Float (double-precision)" :default -90.0) (Right :type "Float (double-precision)" :default 90.0) (Path :type "Float (double-precision)"))
  (`|ExecutionSequence`
    (:`then_0`
      ;[1 1 1] Randomize speed, animation speed
      (`TimelineComponent.SetPlayRate` (`self.RotationTimeline`) (/ 1.0 (`KismetMathLibrary.RandomFloatInRange` 0.1 (`self.TurnMaxDuration`))))
      (set `self.MaxSpeed` (`KismetMathLibrary.RandomFloatInRange` 1.0 (`self.MaxSpeed`))))
    (:`then_1`
      ;[1 1 1] Randomly decide facing direction (Left/Right). Factor in tile rotation
      (if (`KismetMathLibrary.RandomBool`)
        (set `self.MaxSpeed` (* -1 (`self.MaxSpeed`)))
        (set `local.Path` (`local.Left`))
        (else
          (set `local.Path` (`local.Right`))))
      (bind _output_get (set `self.FacingDirection` (`KismetMathLibrary.MakeRotator` (`self.TileRotationY`) 0.0 (`local.Path`))))
      (`SceneComponent.K2_SetRelativeRotation` (`self.Animal`) _output_get false false))))

(fn `UserConstructionScript`
  (bind _size (`self.Size`))
  ;[1 1 1] Apply size scaling
  (`SceneComponent.SetWorldScale3D` (`self.Animal`) _size)
  (`SceneComponent.SetWorldScale3D` (`self.GeneralCollision`) _size))