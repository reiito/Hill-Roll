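; Game mode for the endless slope level, handling track generation, HUD text, results and save data.
; It chains randomly chosen slope tiles by attach transforms, with split tiles that randomly continue one branch and place spikes below the other.
; Each tick it refreshes distance and money text from the player controller; results show a random message and image per lose condition.
; A save slot keeps best distance, held money and instructions-seen state.
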(event `self.ReceiveBeginPlay`
  ;[1 1 1] Setup level
  (`self.SaveGameCheck`)
  (`self.SetupMode` "NewEnumerator0"))

(event `SpawnPlayer`
  (`/Game/Blueprints/Player/BP_PlayerController.SpawnPlayer` (`self.PlayerControllerOReference`)))

(event `self.ReceiveTick`
  (params (DeltaSeconds :type "Float (single-precision)"))
  (`parent.ReceiveTick` DeltaSeconds)
  (`self.UpdateEndlessHUD`))

(fn `AddRandomTile`
  (params (IsSplit :type Boolean))
  (bind _nextspawnpoint (`self.NextSpawnPoint`))
  (bind _tiles (`self.Tiles`))
  (if IsSplit
    (`self.AddSplitTile` _nextspawnpoint)
    (else
      (bind _returnvalue (`|SpawnActorFromClass` (`|GetArrayItem` _tiles (`KismetMathLibrary.RandomIntegerInRange` 0 (`KismetArrayLibrary.Array_LastIndex` _tiles))) _nextspawnpoint "Undefined" "OverrideRootScale" null null))
      (bind _asbp_tile_slope (cast `/Game/Blueprints/Level/BP_Tile_Slope` _returnvalue))
      (bind _transform (`/Game/Blueprints/Level/BP_Tile_Slope.GetAttachTransform` _asbp_tile_slope))
      (set `self.NextSpawnPoint` _transform))))

(fn `AddSplitTile`
  (params (SpawnPoint :type "Transform Structure"))
  (bind _returnvalue (`|SpawnActorFromClass` "/Game/Blueprints/Level/BP_Tile_Slope_Split.BP_Tile_Slope_Split_C" SpawnPoint "Undefined" "OverrideRootScale" null null))
  (if (`KismetMathLibrary.RandomBool`)
    (bind _badattachtransform (`/Game/Blueprints/Level/BP_Tile_Slope_Split.BadAttachTransform` _returnvalue))
    ;[1 1 1] Continue Right
    (set `self.NextSpawnPoint` _badattachtransform)
    (bind _goodattachtransform (`/Game/Blueprints/Level/BP_Tile_Slope_Split.GoodAttachTransform` _returnvalue))
    (`|SpawnActorFromClass` "/Game/Blueprints/Level/BP_Tile_Slope_Fail_Spikes.BP_Tile_Slope_Fail_Spikes_C" (`KismetMathLibrary.Conv_VectorToTransform` (`KismetMathLibrary.TransformLocation` _goodattachtransform (`KismetMathLibrary.MakeVector` 0.0 0.0 (`self.LowerSpikes`)))) "Undefined" "OverrideRootScale" null null)
    (else
      ;[1 1 1] Continue Left
      (set `self.NextSpawnPoint` _goodattachtransform)
      (`|SpawnActorFromClass` "/Game/Blueprints/Level/BP_Tile_Slope_Fail_Spikes.BP_Tile_Slope_Fail_Spikes_C" (`KismetMathLibrary.Conv_VectorToTransform` (`KismetMathLibrary.TransformLocation` _badattachtransform (`KismetMathLibrary.MakeVector` 0.0 0.0 (`self.LowerSpikes`)))) "Undefined" "OverrideRootScale" null null)
      (`/Game/Blueprints/Level/BP_Tile_Slope_Split.ChangeSpikeSign` _returnvalue)))
  (bind _returnvalue_2 (`|SpawnActorFromClass` "/Game/Blueprints/Level/BP_Tile_Slope.BP_Tile_Slope_C" (`self.NextSpawnPoint`) "Undefined" "OverrideRootScale" null null))
  (bind _transform (`/Game/Blueprints/Level/BP_Tile_Slope.GetAttachTransform` _returnvalue_2))
  (set `self.NextSpawnPoint` _transform))

(fn `AddStartTile`
  (bind _returnvalue (`|SpawnActorFromClass` "/Game/Blueprints/Level/BP_Tile_Slope_Start.BP_Tile_Slope_Start_C" (`self.NextSpawnPoint`) "Undefined" "OverrideRootScale" null null))
  (bind _transform (`/Game/Blueprints/Level/BP_Tile_Slope.GetAttachTransform` _returnvalue))
  (set `self.NextSpawnPoint` _transform))

(fn `CreateEndlessLevel`
  (`self.AddStartTile`)
  (for _ (range (+ (`self.StartTiles`) 1))
    (`self.AddRandomTile` false)))

(fn `CreateSaveReference`
  ;[1 1 1] Create instance of save game reference, containing saved data
  (bind _returnvalue (`GameplayStatics.CreateSaveGameObject` "/Game/Blueprints/BP_SaveGame.BP_SaveGame_C"))
  (bind _output_get (set `self.SaveGameReference` _returnvalue))
  (set `/Game/Blueprints/BP_SaveGame.GreatestDistance` (`self.DisplayedGreatestDistance`) _output_get)
  (set `/Game/Blueprints/BP_SaveGame.InstructionsSeen` (`self.SeenInstructions`) (`self.SaveGameReference`))
  (set `/Game/Blueprints/BP_SaveGame.MoneyHeld` (`self.DisplayedHeldMoney`) (`self.SaveGameReference`)))

(fn `LoadGame`
  (bind _returnvalue (`GameplayStatics.LoadGameFromSlot` (`self.saveSlot`)))
  (bind _asbp_save_game (cast `/Game/Blueprints/BP_SaveGame` _returnvalue))
  (set `self.SeenInstructions` (`/Game/Blueprints/BP_SaveGame.InstructionsSeen` _asbp_save_game))
  (set `self.DisplayedGreatestDistance` (`/Game/Blueprints/BP_SaveGame.GreatestDistance` _asbp_save_game))
  (set `self.DisplayedHeldMoney` (`/Game/Blueprints/BP_SaveGame.MoneyHeld` _asbp_save_game)))

(fn `SaveGame`
  (`self.CreateSaveReference`)
  (`self.SaveGreatestDistance`)
  (`self.SaveMoneyEarned`)
  (`GameplayStatics.SaveGameToSlot` (`self.SaveGameReference`) (`self.saveSlot`)))

(fn `SaveGameCheck`
  (`|ExecutionSequence`
    (:`then_0`
      ;[1 1 1] Check save slot to see if save game exists
      (bind _returnvalue (`GameplayStatics.DoesSaveGameExist` (`self.SaveSlot`)))
      (if _returnvalue
        ;;[1 1 1] Save exists, load data
        (`self.LoadGame`)
        (else
          ;;[1 1 1] No saved game exists, set default values
          (set `self.SeenInstructions` false)
          (set `self.DisplayedGreatestDistance` 0)
          (set `self.DisplayedHeldMoney` 0))))
    (:`then_1`
      ;[1 1 1] Set HUD variables to that of loaded/default values
      (`self.UpdateHUDSavedVariables` true true))))

(fn `SaveGreatestDistance`
  (locals (ReachedDistance :type Integer))
  ;[1 1 1] Check whether distance reached is higher than saved distance, if so update it
  (bind _output_get (set `local.ReachedDistance` (`/Game/Blueprints/Player/BP_PlayerController.PlayerDistanceRef` (`self.PlayerControllerOReference`))))
  (if (> _output_get (`self.DisplayedGreatestDistance`))
    ;;[1 1 1] Save new distance reached
    (bind _output_get_2 (set `/Game/Blueprints/BP_SaveGame.GreatestDistance` _output_get (`self.SaveGameReference`)))
    ;;[1 1 1] Update for current display
    (set `self.DisplayedGreatestDistance` _output_get_2)
    (`self.UpdateHUDSavedVariables` true)))

(fn `SaveMoneyEarned`
  ;[1 1 1] Update HUD to show total held money
  (bind _output_get (set `self.DisplayedHeldMoney` (+ (`/Game/Blueprints/Player/BP_PlayerController.PlayerMoneyEarnedRef` (`self.PlayerControllerOReference`)) (`self.DisplayedHeldMoney`))))
  (`self.UpdateHUDSavedVariables` false true)
  ;[1 1 1] Update to save
  (set `/Game/Blueprints/BP_SaveGame.MoneyHeld` _output_get (`self.SaveGameReference`)))

(fn `SetDemiseImage`
  (params (Image :type "Texture2D Object Reference"))
  ;[1 1 1] Create slatebrush with attached image and size specified
  (set `self.DemiseBrushRef` (make `SlateBrush` (`self.DemiseImageSize`) (struct) (struct :`SpecifiedColor` (struct :`R` 1.0 :`G` 1.0 :`B` 1.0 :`A` 1.0) :`ColorUseRule` "UseColor_Specified") Image)))

(fn `SetLoseCaseText`
  (switch `string` (`/Game/Blueprints/Player/BP_PlayerController.PlayerLoseCondition` (`self.PlayerControllerOReference`))
    (:`Animal`
      ;[1 1 1] Select random message matching lose case
      (set `self.PlayerLoseCaseText` (`/Game/Blueprints/BP_Macros.SelectRandomCollisionMessage` (`self.AnimalPrefix`) (`self.AnimalMessages`)))
      ;[1 1 1] Choose matching image
      (`self.SetDemiseImage` "/Game/HUD/Images/Demise/Animal.Animal"))
    (:`Rock`
      (set `self.PlayerLoseCaseText` (`/Game/Blueprints/BP_Macros.SelectRandomCollisionMessage` (`self.RockPrefix`) (`self.RockMessages`)))
      (`self.SetDemiseImage` "/Game/HUD/Images/Demise/Rock.Rock"))
    (:`Tree`
      (set `self.PlayerLoseCaseText` (`/Game/Blueprints/BP_Macros.SelectRandomCollisionMessage` (`self.TreePrefix`) (`self.TreeMessages`)))
      (`self.SetDemiseImage` "/Game/HUD/Images/Demise/Tree.Tree"))
    (:`ZeroVelocity`
      (set `self.PlayerLoseCaseText` (`/Game/Blueprints/BP_Macros.SelectRandomCollisionMessage` (`self.ZeroVelocityPrefix`) (`self.ZeroVelocityMessages`)))
      (`self.SetDemiseImage` "/Game/HUD/Images/Demise/ZeroVelocity.ZeroVelocity"))
    (:`Falling`
      (set `self.PlayerLoseCaseText` (`/Game/Blueprints/BP_Macros.SelectRandomCollisionMessage` (`self.FallingPrefix`) (`self.FallingMessages`)))
      (`self.SetDemiseImage` "/Game/HUD/Images/Demise/Falling.Falling"))
    (:`Backwards`
      (set `self.PlayerLoseCaseText` (`/Game/Blueprints/BP_Macros.SelectRandomCollisionMessage` (`self.BackwardsPrefix`) (`self.BackwardsMessages`)))
      (`self.SetDemiseImage` "/Game/HUD/Images/Demise/Backwards.Backwards"))
    (:`Spike`
      (set `self.PlayerLoseCaseText` (`/Game/Blueprints/BP_Macros.SelectRandomCollisionMessage` (`self.SpikePrefix`) (`self.SpikeMessages`)))
      (`self.SetDemiseImage` "/Game/HUD/Images/Demise/Spikes.Spikes"))
    (:`Water`
      (set `self.PlayerLoseCaseText` (`/Game/Blueprints/BP_Macros.SelectRandomCollisionMessage` (`self.WaterPrefix`) (`self.WaterMessages`)))
      (`self.SetDemiseImage` "/Game/HUD/Images/Demise/Water.Water"))))

(fn `ToggleResults`
  (`self.SetLoseCaseText`)
  (bind _asbp_hud_endless (cast `/Game/HUD/BP_HUD_Endless` (`self.HUDOReference`)))
  (`/Game/HUD/BP_HUD_Endless.ViewResults` _asbp_hud_endless))

(fn `UpdateEndlessHUD`
  (bind _playermoneytallyref (`/Game/Blueprints/Player/BP_PlayerController.PlayerMoneyTallyRef` (`self.PlayerControllerOReference`)))
  (bind _output_count (break `/Game/Data/STRUCT_Tally` (`|GetArrayItem` _playermoneytallyref 1)))
  (bind _output_count_2 (break `/Game/Data/STRUCT_Tally` (`|GetArrayItem` _playermoneytallyref 2)))
  (bind _output_count_3 (break `/Game/Data/STRUCT_Tally` (`|GetArrayItem` _playermoneytallyref)))
  ;[1 1 1] Distance reached
  (set `self.PlayerDistanceTravelledText` (`/Game/Blueprints/BP_Macros.DistanceToText` (`/Game/Blueprints/Player/BP_PlayerController.PlayerDistanceRef` (`self.PlayerControllerOReference`))))
  ;[1 1 1] Money picked up
  (set `self.PlayerSmallMoneyText` (`/Game/Blueprints/BP_Macros.IntegerToTally` _output_count_3))
  (set `self.PlayerMediumMoneyText` (`/Game/Blueprints/BP_Macros.IntegerToTally` _output_count))
  (set `self.PlayerLargeMoneyText` (`/Game/Blueprints/BP_Macros.IntegerToTally` _output_count_2))
  (set `self.PlayerEarnedMoneyText` (`KismetTextLibrary.Conv_IntToText` (`/Game/Blueprints/Player/BP_PlayerController.PlayerMoneyEarnedRef` (`self.PlayerControllerOReference`)))))

(fn `UpdateHUDSavedVariables`
  (params (GreatestDistance :type Boolean) (MoneyHeld :type Boolean))
  (`|ExecutionSequence`
    (:`then_0`
      (if (`local.GreatestDistance`)
        (set `self.PlayerGreatestDistance` (`/Game/Blueprints/BP_Macros.DistanceToText` (`self.DisplayedGreatestDistance`)))))
    (:`then_1`
      (if (`local.MoneyHeld`)
        (set `self.PlayerHeldMoneyText` (`KismetTextLibrary.Conv_IntToText` (`self.DisplayedHeldMoney`)))))))

(fn `UserConstructionScript`
  (`parent.UserConstructionScript`))