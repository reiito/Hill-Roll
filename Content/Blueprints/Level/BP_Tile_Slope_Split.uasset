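; Level tile for a sloped fork, offering a good path and a bad path as attach points for what follows.
; Construction spawns flora, clouds and a random number of trees in left and right boxes, then sets a fixed actor rotation.
; It then caches world transforms from AttachPoint and BadPath as the good and bad attach transforms.
; A separate function swaps the spike sign to its right-hand mesh, and SpawnFenceLine is empty.
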(fn `ChangeSpikeSign`
  (`StaticMeshComponent.SetStaticMesh` (`self.SpikeSign`) "/Game/Models/Level/SpikeSignRight.SpikeSignRight"))

(fn `SetBadPath`
  (set `self.BadAttachTransform` (`SceneComponent.K2_GetComponentToWorld` (`self.BadPath`))))

(fn `SetGoodPath`
  (set `self.GoodAttachTransform` (`SceneComponent.K2_GetComponentToWorld` (`self.AttachPoint`))))

(fn `SpawnFenceLine`)

(fn `SpawnSplitTrees`
  (params (Box :type "BoxComponent Object Reference"))
  (locals (MinTrees :type Integer :default 5) (MaxTrees :type Integer :default 10))
  (for _ (range (`KismetMathLibrary.RandomIntegerInRange` (`local.MinTrees`) (`local.MaxTrees`)))
    (bind _location (`self.SpawnRandomLocation` Box))
    (`AddComponent|NODE_AddChildActorComponent-2` :`RelativeTransform` _location)))

(fn `UserConstructionScript`
  (locals (FenceSegments :type Integer :default 2))
  (set `self.NumFlora` 50)
  (`self.SpawnFlora`)
  (`self.SpawnSplitTrees` (`self.LeftTrees`))
  (`self.SpawnSplitTrees` (`self.RightTrees`))
  (`self.SpawnClouds` 10)
  (`self.K2_SetActorRotation` (struct :`Pitch` -20.0))
  (`self.SetGoodPath`)
  (`self.SetBadPath`))