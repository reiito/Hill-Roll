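; BP_Player_Endless is the player for an endless mode, scored by the farthest X distance travelled from the start point.
; It extends parent player logic, updating the score each tick after launch until restart is allowed.
; Hits store the surface's pitch, which selects a normal or steep spring arm angle that the camera eases toward.
; The R key restarts the level once CanRestart is set.
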(event `self.DestroyPlayer`
  (params (DelayTime :type "Float (single-precision)"))
  (`parent.DestroyPlayer` DelayTime))

(event `Key|R`
  (params (Key :type "Key Structure"))
  ;[1 1 1] Enable restarting, only when results have been seen (set by event dispatcher)
  (:`Pressed`
    (if (`self.CanRestart`)
      (`KismetSystemLibrary.ExecuteConsoleCommand` "RestartLevel"))))

(event `self.ReceiveHit`
  (params (MyComp :type "PrimitiveComponent Object Reference") (Other :type "Actor Object Reference") (OtherComp :type "PrimitiveComponent Object Reference") (bSelfMoved :type Boolean) (HitLocation :type "Vector Structure") (HitNormal :type "Vector Structure") (NormalImpulse :type "Vector Structure") (Hit :type "HitResult Structure (by ref)"))
  (bind (_returnvalue_roll _returnvalue_pitch) (`KismetMathLibrary.BreakRotator` (`self.K2_GetActorRotation` Other)))
  (`parent.ReceiveHit` null null null false (0.0 0.0 0.0) (0.0 0.0 0.0) (0.0 0.0 0.0) Hit)
  (set `self.GroundAngle` _returnvalue_pitch))

(event `self.ReceiveBeginPlay`
  (`parent.ReceiveBeginPlay`)
  ;[1 1 1] Set starting position, for calculating distance travelled
  (bind _output_get (set `self.StartLocation` (`SceneComponent.K2_GetComponentLocation` (`self.Body`))))
  (set `self.CurrentLocation` _output_get))

(event `self.ReceiveTick`
  (params (DeltaSeconds :type "Float (single-precision)"))
  (`parent.ReceiveTick` DeltaSeconds)
  (`self.RotateSpringArm` DeltaSeconds)
  ;[1 1 1] Once launched and not viewing results (case of falling), start adding to score
  (if (and (`self.Launched`) (not (`self.CanRestart`)))
    (`self.CalculateScore`)))

(fn `CalculateScore`
  (bind _returnvalue_x (`KismetMathLibrary.BreakVector` (- (`self.StartLocation`) (`self.CurrentLocation`))))
  (bind _returnvalue (`KismetMathLibrary.Round` (* _returnvalue_x -1.0)))
  ;[1 1 1] Score based on distance travelled, how far player moved
  ;;[1 1 1] Update current position as opposed to where they launched
  (set `self.CurrentLocation` (`SceneComponent.K2_GetComponentLocation` (`self.Body`)))
  (if (> _returnvalue (`self.DistanceTravelled`))
    (set `self.DistanceTravelled` _returnvalue)))

(fn `RotateSpringArm`
  (params (DeltaTime :type "Float (double-precision)"))
  (bind _springarm (`self.SpringArm`))
  (if (`KismetMathLibrary.NearlyEqual_FloatFloat` (`self.GroundAngle`) -15.0 0.01)
    (set `self.SpringRot` (`KismetMathLibrary.MakeRotator` 0.0 (`self.NormalAngle`)))
    (else
      (set `self.SpringRot` (`KismetMathLibrary.MakeRotator` 0.0 (`self.SteepAngle`)))))
  (`SceneComponent.K2_SetWorldRotation` _springarm (`KismetMathLibrary.RLerp` (`SceneComponent.K2_GetComponentRotation` _springarm) (`self.SpringRot`) (* DeltaTime (`self.CameraSpeed`))) false false))

(fn `UserConstructionScript`
  (`parent.UserConstructionScript`))