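; BP_Flora is a decorative plant actor that flattens the first time something overlaps it.
; The construction script gives the Flora mesh a random pick from FloraArray.
; A DoOnce on the overlap event plays the FlattenAnimation timeline, whose alpha feeds Flatten.
; Flatten lerps world rotation from its current value toward a fixed target, so the blend compounds each update.
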(event `self.Flora.OnComponentBeginOverlap`
  (params (OverlappedComponent :type "PrimitiveComponent Object Reference") (OtherActor :type "Actor Object Reference") (OtherComp :type "PrimitiveComponent Object Reference") (OtherBodyIndex :type Integer) (bFromSweep :type Boolean) (SweepResult :type "HitResult Structure (by ref)"))
  (`/Engine/EditorBlueprintResources/StandardMacros.DoOnce` false
    (:`Completed`
      (bind (_direction _alpha) (`Timeline|FlattenAnimation`)
        (:`Update`
          (`self.Flatten` _alpha))))))

(fn `Flatten`
  (params (LerpAlpha :type "Float (double-precision)"))
  (`SceneComponent.K2_SetWorldRotation` (`self.Flora`) (`KismetMathLibrary.RLerp` (`SceneComponent.K2_GetComponentRotation` (`self.Flora`)) (struct :`Pitch` 90.0) LerpAlpha) false false))

(fn `UserConstructionScript`
  (`StaticMeshComponent.SetStaticMesh` (`self.Flora`) (`/Game/Blueprints/BP_Macros.SelectRandomFromArray` (`self.FloraArray`))))