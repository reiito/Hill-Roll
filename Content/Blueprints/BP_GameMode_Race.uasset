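; Race game mode that spawns the starting player and times the run from the moment that player launches.
; BeginPlay sets up the mode, and SpawnStartingPlayer binds StartLevel to the launch event of the referenced controller's race player.
; StartLevel disables swinging on that controller and starts the timer.
; A Timeline serves as the clock, updating elapsed time and its text form until stopped.
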(event `self.ReceiveBeginPlay`
  (`self.SetupMode` "NewEnumerator1"))

(event `StartGameTimer`
  ;[1 1 1] Game Timer
  (bind (_direction _timepassed) (`Timeline|Timeline_0` :!label _label)
    (:`Update`
      (bind _output_get (set `self.elapsedTime` _timepassed))
      (set `self.elapsedTimeText` (`/Game/Blueprints/BP_Macros.TimeToText` _output_get)))))

(event `StopGameTimer`
  ;[1 1 1] Game Timer
  (goto _label :!via `Stop`))

(event `SpawnStartingPlayer`
  (bind _playercontrolleroreference (`self.PlayerControllerOReference`))
  ;[1 1 1] Attach to first player only, start game timer
  (`/Game/Blueprints/Player/BP_PlayerController.SpawnPlayer` _playercontrolleroreference)
  (add `/Game/Blueprints/Player/BP_Player.PlayerLaunched` (`/Game/Blueprints/Player/BP_PlayerController.RacePlayerOReference` _playercontrolleroreference) (delegate `StartLevel`)))

(event `StartLevel`
  ;[1 1 1] Attach to first player only, start game timer
  (`self.StartGameTimer`)
  (set `/Game/Blueprints/Player/BP_PlayerController.EnableSwinging` false (`self.PlayerControllerOReference`)))

(fn `UserConstructionScript`
  (`parent.UserConstructionScript`))