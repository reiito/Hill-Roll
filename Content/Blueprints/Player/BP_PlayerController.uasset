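; Player controller for the Endless and Race game types that spawns, possesses and automatically respawns the chosen character.
; It stores the pawn as a mode-specific reference and mirrors its stats each Tick, speed for both modes plus distance and money for Endless.
; When an Endless run finishes, it toggles results, tallies money earned, plays a timeline-driven count-up, allows restarting and saves the game.
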(event `InitializeController`
  (params (SpawnLocation :type "Vector Structure") (ChosenCharacter :type "/Game/Blueprints/Player/BP_Player Class Reference") (GameMode :type "/Game/Blueprints/BP_GameMode Object Reference") (GameType :type "/Game/Data/ENUM_GameType Enum" :default "NewEnumerator0"))
  ;[1 1 1] Initialize on start-up - Set-up Location/Reference/State
  (set `self.SpawnPoint` (`KismetMathLibrary.MakeTransform` SpawnLocation))
  (set `self.PlayerCReference` ChosenCharacter)
  (set `self.GameModeOReference` GameMode)
  (set `self.GameType` GameType))

(event `SpawnPlayer`
  ;[1 1 1] Spawn Player
  (bind _returnvalue (`|SpawnActorFromClass` (`self.PlayerCReference`) (`self.SpawnPoint`) "AlwaysSpawn" "OverrideRootScale" null null))
  (`self.Possess` _returnvalue)
  (add `self.OnDestroyed` _returnvalue (delegate `Respawn`))
  ;[1 1 1] Store type depending on game type
  (`self.SetPlayerType` _returnvalue))

(event `Respawn` :!signature `self.OnDestroyed`
  (params (DestroyedActor :type "Actor Object Reference"))
  ;[1 1 1] Spawn Player
  (`self.SpawnPlayer`))

(event `self.ReceiveTick`
  (params (DeltaSeconds :type "Float (single-precision)"))
  (`self.UpdatePlayerParamReferences`))

(event `SetPlayerType`
  (params (SpawnedPlayer :type "/Game/Blueprints/Player/BP_Player Object Reference"))
  (switch `/Game/Data/ENUM_GameType` (`self.GameType`)
    (:`NewEnumerator0`
      (bind _asbp_player_endless (cast `/Game/Blueprints/Player/BP_Player_Endless` SpawnedPlayer))
      (bind _output_get (set `self.EndlessPlayerOReference` _asbp_player_endless))
      (add `/Game/Blueprints/Player/BP_Player.PlayerFinish` SpawnedPlayer (delegate `ShowResults`)))
    (:`NewEnumerator1`
      (bind _asbp_player_race (cast `/Game/Blueprints/Player/BP_Player_Race` SpawnedPlayer))
      (set `self.RacePlayerOReference` _asbp_player_race))))

(event `ShowResults`
  (params (LoseCondition :type String))
  ;[1 1 1] Show results when player has finished
  (set `self.PlayerLoseCondition` LoseCondition)
  (bind _asbp_game_mode_endless (cast `/Game/Blueprints/BP_GameMode_Endless` (`self.GameModeOReference`)))
  (`/Game/Blueprints/BP_GameMode_Endless.ToggleResults` _asbp_game_mode_endless)
  (`self.TallyCurrencyEarned`)
  (`self.AnimateMoneyEarned`)
  (set `/Game/Blueprints/Player/BP_Player_Endless.CanRestart` true (stale `SetPlayerType` _output_get))
  (`/Game/Blueprints/BP_GameMode_Endless.SaveGame` _asbp_game_mode_endless))

(event `AnimateMoneyEarned`
  ;[1 1 1] Perform lerp animation to show money totals count upwards from 0
  (`TimelineComponent.SetPlayRate` (`self.MoneyEarnedAnimation`) (`self.MoneyAnimationPlaySpeed`))
  (bind (_direction _moneyearnedalpha) (`Timeline|MoneyEarnedAnimation`)
    (:`Update`
      (set `self.PlayerAnimatedMoneyEarnedRef` (`KismetMathLibrary.FTrunc` (`KismetMathLibrary.Lerp` 0.0 (`KismetMathLibrary.Conv_IntToDouble` (`self.PlayerMoneyEarnedRef`)) _moneyearnedalpha))))))

(fn `TallyCurrencyEarned`
  (locals (MoneyEarned :type Integer))
  ;[1 1 1] Add up tallies for money earned, their count by their value and add to total earned
  (for _array_element (`self.PlayerMoneyTallyRef`)
    (bind (_count _value) (break `/Game/Data/STRUCT_Tally` _array_element))
    (set `self.PlayerMoneyEarnedRef` (+ (* _count _value) (`self.PlayerMoneyEarnedRef`)))))

(fn `UpdatePlayerParamReferences`
  (bind _endlessplayeroreference (`self.EndlessPlayerOReference`))
  (bind _raceplayeroreference (`self.RacePlayerOReference`))
  ;[1 1 1] Store parameters depending on game type. Only do so when valid
  (switch `/Game/Data/ENUM_GameType` (`self.GameType`)
    (:`NewEnumerator0`
      ;[1 1 1] Endless
      (`/Engine/EditorBlueprintResources/StandardMacros.IsValid` _endlessplayeroreference
        (:`Is Valid`
          (set `self.PlayerSpeedRef` (`/Game/Blueprints/Player/BP_Player.Speed` _endlessplayeroreference))
          (set `self.PlayerDistanceRef` (`/Game/Blueprints/Player/BP_Player_Endless.DistanceTravelled` _endlessplayeroreference))
          (set `self.PlayerMoneyEarnedRef` (`/Game/Blueprints/Player/BP_Player.MoneyEarned` _endlessplayeroreference))
          (set `self.PlayerMoneyTallyRef` (`/Game/Blueprints/Player/BP_Player.MoneyTally` _endlessplayeroreference)))))
    (:`NewEnumerator1`
      ;[1 1 1] Race
      (`/Engine/EditorBlueprintResources/StandardMacros.IsValid` _raceplayeroreference
        (:`Is Valid`
          (set `self.PlayerSpeedRef` (`/Game/Blueprints/Player/BP_Player.Speed` _raceplayeroreference)))))))

(fn `UserConstructionScript`)