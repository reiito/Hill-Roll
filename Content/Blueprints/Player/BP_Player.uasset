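; Player pawn for a physics game where the character swings, launches by breaking hand constraints, then rolls through a level collecting money.
; Axis input follows state: swing or reposition before launch, then change speed or steer by scaling arm and leg shapes.
; Per-frame ground traces toggle rolling and physical-animation ragdoll.
; Stalling, falling, obstacle body hits or Water overlap end trigger delayed loss; limb hits briefly disable that limb's collision.
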(event `Key|Escape`
  (params (Key :type "Key Structure"))
  (:`Pressed`
    (`KismetSystemLibrary.QuitGame` null "Quit")))

(event `self.ReceiveBeginPlay`
  ;[1 1 1] Begin Play and add starting impulse
  (`self.Initialize`)
  (`PrimitiveComponent.AddImpulse` (`self.Body`) (`self.SwingForce`) "None" false))

(event `InputAxis|MovementLeftRight`
  (params (AxisValue :type "Float (single-precision)"))
  ;[1 1 1] Key input
  (`self.LeftRightMovement` AxisValue))

(event `self.ReceiveTick`
  (params (DeltaSeconds :type "Float (single-precision)"))
  ;[1 1 1] Update per frame
  (`self.UpdatePlayer`))

(event `InputAxis|MovementUpDown`
  (params (AxisValue :type "Float (single-precision)"))
  ;[1 1 1] Key input
  (`self.UpDownMovement` AxisValue))

(event `InputAction|LaunchJump`
  (params (Key :type "Key Structure"))
  ;[1 1 1] Key input
  (:`Pressed`
    (`/Engine/EditorBlueprintResources/StandardMacros.DoOnce` false
      (:`Completed`
        (`self.Launch`)))))

(event `DestroyPlayer`
  (params (DelayTime :type "Float (double-precision)"))
  ;[1 1 1] Destroy player, notify level over
  (`KismetSystemLibrary.Delay` DelayTime)
  (`self.PlayerFinish` (`self.LoseCase`)))

(event `ZeroVelocityRespawnCheck`
  ;[1 1 1] Respawn check cases
  ;;[1 1 1] 1. Forward velocity < 1. Player has slowed down to a halt and cannot move further. Force a respawn
  (bind _returnvalue (`PrimitiveComponent.GetPhysicsLinearVelocity` (`self.Body`) "None"))
  (if (and (> (.x _returnvalue) 0.0) (< (.x _returnvalue) (`self.MinLinearVelocity`)))
    (`self.DisableAndRagdoll`)
    (set `self.LoseCase` "ZeroVelocity")
    (`self.DestroyPlayer` (`self.RespawnTime`))))

(event `Key|T`
  (params (Key :type "Key Structure"))
  ;[1 1 1] REMOVE AT END -- DEBUG/TESTING
  (:`Pressed`
    (`SceneComponent.SetHiddenInGame` (`self.Arms`) (`self.HideShapes`) false)
    (`SceneComponent.SetHiddenInGame` (`self.Legs`) (`self.HideShapes`) false)
    (`SceneComponent.SetHiddenInGame` (`self.Body`) (`self.HideShapes`) false)
    (set `self.HideShapes` (not (`self.HideShapes`)))))

(event `OutOfBoundsRespawnCheck`
  ;[1 1 1] Respawn check cases
  ;;[1 1 1] 2. Player has fallen out of bounds of the map, factor in time spent falling added with default respawn time
  (bind _returnvalue (`PrimitiveComponent.GetPhysicsLinearVelocity` (`self.Body`) "None"))
  (if (< (.z _returnvalue) (`self.OutOfBoundsZVelocity`))
    (set `self.LoseCase` "Falling")
    (`self.DestroyPlayer` (+ (`self.RespawnTime`) (`self.OutOfBoundsRespawnTime`)))))

(event `Key|H`
  (params (Key :type "Key Structure"))
  ;[1 1 1] REMOVE AT END -- DEBUG/TESTING
  (:`Pressed`
    (`SceneComponent.SetVisibility` (`self.Model`) (`self.HideModel`) false)
    (set `self.HideModel` (not (`self.HideModel`)))))

(event `self.ReceiveActorBeginOverlap`
  (params (OtherActor :type "Actor Object Reference"))
  (`self.CheckMoneyPickup` OtherActor))

(event `self.ReceiveHit`
  (params (MyComp :type "PrimitiveComponent Object Reference") (Other :type "Actor Object Reference") (OtherComp :type "PrimitiveComponent Object Reference") (bSelfMoved :type Boolean) (HitLocation :type "Vector Structure") (HitNormal :type "Vector Structure") (NormalImpulse :type "Vector Structure") (Hit :type "HitResult Structure (by ref)"))
  ;[1 1 1] Collision and overlap detection
  (bind _hascollided (`self.CollidedWithTagged` "Ground" Hit))
  (if _hascollided
    (`/Engine/EditorBlueprintResources/StandardMacros.DoOnce` false
      (:`Completed`
        (`self.FirstLanding`)))))

(event `self.Body.OnComponentHit`
  (params (HitComponent :type "PrimitiveComponent Object Reference") (OtherActor :type "Actor Object Reference") (OtherComp :type "PrimitiveComponent Object Reference") (NormalImpulse :type "Vector Structure") (Hit :type "HitResult Structure (by ref)"))
  ;[1 1 1] Collision and overlap detection
  (bind _hascollided (`self.CollidedWithTagged` "Obstacle" Hit))
  (if _hascollided
    (`self.DisableAndRagdoll`)
    ;;[1 1 1] Get collided second tag to determine specific collided object
    (bind _tag (`/Game/Blueprints/BP_Macros.GetComponentTag` 1 (`.HitComponent` (`GameplayStatics.BreakHitResult` Hit)))
      (:`__`
        (set `self.LoseCase` _tag)
        (`self.DestroyPlayer` (`self.RespawnTime`))))))

(event `self.Arms.OnComponentHit`
  (params (HitComponent :type "PrimitiveComponent Object Reference") (OtherActor :type "Actor Object Reference") (OtherComp :type "PrimitiveComponent Object Reference") (NormalImpulse :type "Vector Structure") (Hit :type "HitResult Structure (by ref)"))
  ;[1 1 1] Collision and overlap detection
  ;;[1 1 1] Hitting obstacles with either arms/legs player is slowed down for hitting the obstacle
  (bind _hascollided (`self.CollidedWithTagged` "Obstacle" Hit))
  (if _hascollided
    (`self.ToggleLimbCollision` (`self.Arms`) 1.0)))

(event `self.Legs.OnComponentHit`
  (params (HitComponent :type "PrimitiveComponent Object Reference") (OtherActor :type "Actor Object Reference") (OtherComp :type "PrimitiveComponent Object Reference") (NormalImpulse :type "Vector Structure") (Hit :type "HitResult Structure (by ref)"))
  ;[1 1 1] Collision and overlap detection
  ;;[1 1 1] Hitting obstacles with either arms/legs player is slowed down for hitting the obstacle
  (bind _hascollided (`self.CollidedWithTagged` "Obstacle" Hit))
  (if _hascollided
    (`self.ToggleLimbCollision` (`self.Legs`) 1.0)))

(event `self.Body.OnComponentEndOverlap`
  (params (OverlappedComponent :type "PrimitiveComponent Object Reference") (OtherActor :type "Actor Object Reference") (OtherComp :type "PrimitiveComponent Object Reference") (OtherBodyIndex :type Integer))
  ;[1 1 1] Collision and overlap detection
  (bind _tag (`/Game/Blueprints/BP_Macros.GetComponentTag` 0 OtherComp)
    (:`__`
      (if (`KismetStringLibrary.EqualEqual_StrStr` _tag "Water")
        (set `self.LoseCase` _tag)
        (`self.DisableAndRagdoll`)
        (`self.DestroyPlayer` (`self.RespawnTime`))))))

(event `ToggleLimbCollision`
  (params (Limb :type "StaticMeshComponent Object Reference") (Duration :type "Float (double-precision)"))
  ;[1 1 1] Turn off collision for brief time then turn back on
  (`PrimitiveComponent.SetCollisionResponseToChannel` Limb "ECC_GameTraceChannel2" "ECR_Ignore")
  (`KismetSystemLibrary.Delay` Duration)
  (`PrimitiveComponent.SetCollisionResponseToChannel` Limb "ECC_GameTraceChannel2" "ECR_Block"))

(fn `AdjustSpeed`
  (params (InputAxis :type "Float (double-precision)"))
  (if (> InputAxis 0.0)
    ;[1 1 1] Speed up - grow limbs
    (`self.ScaleAndAnimateLimb` (`self.Arms`) true "NewEnumerator1")
    (`self.ScaleAndAnimateLimb` (`self.Legs`) true)
    (else
      ;[1 1 1] Slow down - shrink limbs
      (`self.ScaleAndAnimateLimb` (`self.Arms`) false "NewEnumerator1")
      (`self.ScaleAndAnimateLimb` (`self.Legs`)))))

(fn `ApplyRotationToModel`
  ;[1 1 1] Inherit parameters from parent, only rotate whilst rolling and when ragdolling, ensure location matches up to body after landing
  (if (`|EnumEquality` (`self.CurrentState`) "NewEnumerator1")
    (`SceneComponent.K2_SetWorldRotation` (`self.Model`) (`SceneComponent.K2_GetComponentRotation` (`self.Body`)) false false)
    (`SceneComponent.K2_SetWorldLocation` (`self.Model`) (`SceneComponent.K2_GetComponentLocation` (`self.Body`)) false false)))

(fn `CheckMoneyPickup`
  (params (MoneyPickedUp :type "Actor Object Reference"))
  (bind _moneytally (`self.MoneyTally`))
  (bind _output_count (break `/Game/Data/STRUCT_Tally` (`|GetArrayItem` _moneytally 2)))
  (bind _output_count_2 (break `/Game/Data/STRUCT_Tally` (`|GetArrayItem` _moneytally)))
  (bind _output_count_3 (break `/Game/Data/STRUCT_Tally` (`|GetArrayItem` _moneytally 1)))
  ;[1 1 1] If money overlapped, pick it up, update tally and money earned
  (bind _asbp_pickup_money (cast `/Game/Blueprints/Level/Pickups/BP_Pickup_Money` MoneyPickedUp))
  (set `self.MoneyEarned` (+ (`self.MoneyEarned`) (`/Game/Blueprints/Level/Pickups/BP_Pickup_Money.Value` _asbp_pickup_money)))
  (switch `/Game/Data/ENUM_MoneyValues` (`/Game/Blueprints/Level/Pickups/BP_Pickup_Money.Type` _asbp_pickup_money)
    (:`NewEnumerator0`
      (`/Engine/EditorBlueprintResources/StandardMacros.IncrementInt` _output_count_2
        (:`  `
          _)))
    (:`NewEnumerator1`
      (`/Engine/EditorBlueprintResources/StandardMacros.IncrementInt` _output_count_3
        (:`  `
          _)))
    (:`NewEnumerator2`
      (`/Engine/EditorBlueprintResources/StandardMacros.IncrementInt` _output_count
        (:`  `
          _))))
  (`self.K2_DestroyActor` (`local.MoneyPickedUp`)))

(fn `CheckRequireRespawn`
  (locals (ZeroVelocityDelayCheck :type "Float (double-precision)" :default 2.0) (ZeroVelocityRespawnTime :type "Float (double-precision)" :default 1.0))
  ;[1 1 1] Cases explained in event graph
  (`|ExecutionSequence`
    (:`then_0`
      (`self.ZeroVelocityRespawnCheck`))
    (:`then_1`
      (`self.OutOfBoundsRespawnCheck`))))

(fn `CollidedWithTagged`
  (params (Tag :type String) (Hit :type "HitResult Structure"))
  (returns (HasCollided :type Boolean))
  (locals (Result :type Boolean))
  ;[1 1 1] Check whether tag of hit object matches requested tag
  (bind _tag (`/Game/Blueprints/BP_Macros.GetComponentTag` 0 (`.HitComponent` (`GameplayStatics.BreakHitResult` Hit)))
    (:`__`
      ;[1 1 1] Send out result
      (if (`KismetStringLibrary.EqualEqual_StrStr` _tag Tag)
        (set `local.Result` true)
        (else
          (set `local.Result` false)))
      (return (`local.Result`)))))

(fn `DisableAndRagdoll`
  (set `self.Respawning` true)
  ;[1 1 1] Disable physics simulation on body, prevent further movement
  (`PrimitiveComponent.SetSimulatePhysics` (`self.Body`) false)
  ;[1 1 1] Disable movement input
  (set `self.CurrentState` "NewEnumerator4")
  ;[1 1 1] Turn on ragdolling
  (`self.ToggleRagdoll` true))

(fn `FirstLanding`
  ;[1 1 1] Enable rotations
  (`PrimitiveComponent.SetConstraintMode` (`self.Body`) "None")
  (set `self.Landed` true))

(fn `Initialize`
  (`|ExecutionSequence`
    (:`then_0`
      ;[1 1 1] Limit angular rotation
      (`PrimitiveComponent.SetPhysicsMaxAngularVelocityInDegrees` (`self.Arms`) (`self.MaxAngularVelocity`) false "None")
      (`PrimitiveComponent.SetPhysicsMaxAngularVelocityInDegrees` (`self.Legs`) (`self.MaxAngularVelocity`) false "None")
      (`PrimitiveComponent.SetPhysicsMaxAngularVelocityInDegrees` (`self.Body`) (`self.MaxAngularVelocity`) false "None"))
    (:`then_1`
      ;[1 1 1] Setup default limb rotation - arms
      (set `self.LeftArmRotation` (* (`self.ArmStartRotation`) -1.0))
      (set `self.RightArmRotation` (`self.ArmStartRotation`))
      ;[1 1 1] Default limb rotation - legs
      (set `self.LeftLegRotation` (* (`self.LegStartRotation`) -1.0))
      (set `self.RightLegRotation` (`self.LegStartRotation`)))
    (:`then_2`
      ;[1 1 1] Load and apply level parameters pulled from the player controller
      (`self.LoadLevelParameters`)
      (`self.SetupSpringArm`))
    (:`then_3`
      ;[1 1 1] Initialize ragdoll settings
      (`self.SetupRagdoll`))))

(fn `IsAirborne`
  (bind _returnvalue (`SceneComponent.K2_GetComponentLocation` (`self.Body`)))
  ;[1 1 1] Check if in air - Traces line downwards
  (bind (_outhit _returnvalue_2) (`KismetSystemLibrary.LineTraceSingle` _returnvalue (`KismetMathLibrary.MakeVector` (.x _returnvalue) (.y _returnvalue) (- (.z _returnvalue) (`self.LineTraceDistance`))) "TraceTypeQuery1"))
  (if _returnvalue_2
    (set `self.CurrentState` "NewEnumerator1")
    (`self.ToggleRagdoll` false)
    (else
      (set `self.CurrentState` "NewEnumerator3")
      (`self.ToggleRagdoll` true))))

(fn `Launch`
  ;[1 1 1] Release from swinging and notify player controller that player launched
  (set `self.Launched` true)
  (`PhysicsConstraintComponent.BreakConstraint` (`self.P1LeftHandToArms`))
  (`PhysicsConstraintComponent.BreakConstraint` (`self.P1RightHandToArms`))
  (`PhysicsConstraintComponent.BreakConstraint` (`self.P2LeftHandToLegs`))
  (`PhysicsConstraintComponent.BreakConstraint` (`self.P2RightHandToLegs`))
  (`self.PlayerLaunched`))

(fn `LeftRightMovement`
  (params (InputAxis :type "Float (double-precision)"))
  (if (!= InputAxis 0.0)
    (switch `/Game/Data/ENUM_PlayerState` (`self.CurrentState`)
      (:`NewEnumerator0`
        (`self.Reposition` InputAxis))
      (:`NewEnumerator1`
        (`self.Steer` InputAxis)))))

(fn `LoadLevelParameters`
  (locals (RepositionCap :type "Float (double-precision)"))
  (bind _asbp_player_controller (cast `/Game/Blueprints/Player/BP_PlayerController` (`GameplayStatics.GetPlayerController` 0)))
  (set `self.PlayerControllerOReference` _asbp_player_controller)
  ;[1 1 1] Repositioning
  (bind _output_get (set `local.RepositionCap` (`/Game/Blueprints/Player/BP_PlayerController.LevelRepositionCap` (`self.PlayerControllerOReference`))))
  (bind _output_get_2 (set `self.RepositionMax` _output_get))
  (set `self.RepositionMin` (* _output_get_2 -1.0))
  ;[1 1 1] Camera
  (set `self.SpringArmRotation` (`/Game/Blueprints/Player/BP_PlayerController.LevelRotationY` (`self.PlayerControllerOReference`)))
  (set `self.SpringArmLength` (`/Game/Blueprints/Player/BP_PlayerController.PlayerCameraDistance` (`self.PlayerControllerOReference`)))
  ;[1 1 1] Respawning
  (set `self.RespawnTime` (`/Game/Blueprints/Player/BP_PlayerController.PlayerRespawnTime` (`self.PlayerControllerOReference`))))

(fn `Reposition`
  (params (InputAxis :type "Float (double-precision)"))
  (locals (RepositionMade :type "Float (double-precision)"))
  ;[1 1 1] Determine whether repositioning result is in bounds
  (bind _output_get (set `local.RepositionMade` (* InputAxis (`self.RepositionSpeed`))))
  (if (`KismetMathLibrary.InRange_FloatFloat` (+ _output_get (`self.CurrentPositioning`)) (`self.RepositionMin`) (`self.RepositionMax`))
    ;[1 1 1] Shift player left/right and update current positioning
    (`self.K2_AddActorWorldOffset` (`KismetMathLibrary.MakeVector` 0.0 (`local.RepositionMade`)))
    (set `self.CurrentPositioning` (+ (`local.RepositionMade`) (`self.CurrentPositioning`)))))

(fn `RotateLimb`
  (params (Extend :type Boolean) (Limb :type "/Game/Data/ENUM_PlayerLimbs Enum" :default "NewEnumerator0"))
  (locals (Shift :type "Vector Structure") (Direction :type "Float (double-precision)"))
  ;[1 1 1] Determine whether we are moving limb outwards or inwards
  (if Extend
    (set `local.Direction` 1.0)
    (else
      (set `local.Direction` -1.0)))
  ;[1 1 1] Determine which limb to apply the rotation to - Left = Legs, Right = Arms
  (if (`|EnumEquality` (`local.Limb`) "NewEnumerator0")
    (set `local.Shift` (* (`self.LegsRotationShift`) (`local.Direction`)))
    ;[1 1 1] Apply rotations
    (set `self.LeftLegRotation` (`/Game/Blueprints/BP_Macros.AddRotatorAndVector` (`self.LeftLegRotation`) (* (`local.Shift`) -1.0)))
    (set `self.RightLegRotation` (`/Game/Blueprints/BP_Macros.AddRotatorAndVector` (`self.RightLegRotation`) (`local.Shift`)))
    (else
      (set `local.Shift` (* (`self.ArmsRotationShift`) (`local.Direction`)))
      (set `self.LeftArmRotation` (`/Game/Blueprints/BP_Macros.AddRotatorAndVector` (`self.LeftArmRotation`) (`local.Shift`)))
      (set `self.RightArmRotation` (`/Game/Blueprints/BP_Macros.AddRotatorAndVector` (`self.RightArmRotation`) (* (`local.Shift`) -1.0))))))

(fn `ScaleAndAnimateLimb`
  (params (Limb :type "SceneComponent Object Reference") (Grow :type Boolean) (RotatedLimb :type "/Game/Data/ENUM_PlayerLimbs Enum" :default "NewEnumerator0"))
  (locals (UpdatedScale :type "Vector Structure") (AddedScale :type "Vector Structure"))
  ;[1 1 1] Determine whether limb is growing or shrinking
  (if Grow
    (set `local.AddedScale` (`self.RadiusShift`))
    (else
      (set `local.AddedScale` (* (`self.RadiusShift`) -1.0))))
  ;[1 1 1] Follow through when resultant scale is in appropriate range
  (bind _output_get (set `local.UpdatedScale` (+ (`local.AddedScale`) (`SceneComponent.K2_GetComponentScale` (`local.Limb`)))))
  (if (`KismetMathLibrary.InRange_FloatFloat` (.x _output_get) (`self.MinLimbRadiusScale`) (`self.MaxLimbRadiusScale`))
    ;[1 1 1] Apply scaling and rotation of limb
    (`SceneComponent.SetRelativeScale3D` (`local.Limb`) (`local.UpdatedScale`))
    (`self.RotateLimb` (`local.Grow`) (`local.RotatedLimb`))))

(fn `SetupRagdoll`
  (locals (LowOrientationStrength :type "Float (double-precision)" :default 10.0) (LowAngularVelStrength :type "Float (double-precision)" :default 1.0) (HighOrientationStrength :type "Float (double-precision)" :default 100.0) (HighAngularVelStrength :type "Float (double-precision)" :default 10.0))
  (bind _physicalanimationdata (make `PhysicalAnimationData` true (`local.HighOrientationStrength`) (`local.HighAngularVelStrength`)))
  ;[1 1 1] Ragdoll animation setup
  (`PhysicalAnimationComponent.SetSkeletalMeshComponent` (`self.PhysicalAnimation`) (`self.Model`))
  (`PhysicalAnimationComponent.ApplyPhysicalAnimationSettingsBelow` (`self.PhysicalAnimation`) (`self.RagdollBone`) (make `PhysicalAnimationData` true (`local.LowOrientationStrength`) (`local.LowAngularVelStrength`)) true)
  (`PhysicalAnimationComponent.ApplyPhysicalAnimationSettingsBelow` (`self.PhysicalAnimation`) "spine_01" (make `PhysicalAnimationData` true (`local.HighOrientationStrength`) (`local.HighAngularVelStrength`)) true)
  (`PhysicalAnimationComponent.ApplyPhysicalAnimationSettingsBelow` (`self.PhysicalAnimation`) "thigh_l" _physicalanimationdata true)
  (`PhysicalAnimationComponent.ApplyPhysicalAnimationSettingsBelow` (`self.PhysicalAnimation`) "thigh_r" _physicalanimationdata true))

(fn `SetupSpringArm`
  (bind (_returnvalue_roll _returnvalue_pitch _returnvalue_yaw) (`KismetMathLibrary.BreakRotator` (`SceneComponent.K2_GetComponentRotation` (`self.SpringArm`))))
  ;[1 1 1] Setup springarm parameters
  (set `SpringArmComponent.TargetArmLength` (`self.SpringArmLength`) (`self.SpringArm`))
  ;[1 1 1] Add extra rotation to spring arm based on world rotation
  (`SceneComponent.K2_SetWorldRotation` (`self.SpringArm`) (`KismetMathLibrary.MakeRotator` _returnvalue_roll (+ _returnvalue_pitch (`self.SpringArmRotation`)) _returnvalue_yaw) false false))

(fn `Steer`
  (params (InputAxis :type "Float (double-precision)"))
  (locals (SteeredLimb :type "StaticMeshComponent Object Reference") (OpposingLimb :type "StaticMeshComponent Object Reference") (OppositeLimb :type "/Game/Data/ENUM_PlayerLimbs Enum") (Limb :type "/Game/Data/ENUM_PlayerLimbs Enum"))
  (bind _returnvalue_x (`KismetMathLibrary.BreakVector` (`SceneComponent.K2_GetComponentScale` (`local.OpposingLimb`))))
  (if (< InputAxis 0.0)
    ;[1 1 1] Differentiate between limbs currently being rotated (legs/arms), Left = Legs, Right = Arms
    (set `local.Limb` "NewEnumerator0")
    (set `local.SteeredLimb` (`self.Legs`))
    (set `local.OpposingLimb` (`self.Arms`))
    (set `local.OppositeLimb` "NewEnumerator1")
    (else
      (set `local.Limb` "NewEnumerator1")
      (set `local.SteeredLimb` (`self.Arms`))
      (set `local.OpposingLimb` (`self.Legs`))
      (set `local.OppositeLimb` "NewEnumerator0")))
  ;[1 1 1] If opposing limb is smaller than limb base size, grow it to base size, Otherwise shrink steered limb
  (if (< _returnvalue_x (`self.MaxLimbRadiusScale`))
    ;[1 1 1] Apply scaling and rotations
    (`self.ScaleAndAnimateLimb` (`local.OpposingLimb`) true (`local.OppositeLimb`))
    (else
      (`self.ScaleAndAnimateLimb` (`local.SteeredLimb`) false (`local.Limb`)))))

(fn `Swing`
  (params (InputAxis :type "Float (double-precision)"))
  (`PrimitiveComponent.AddImpulse` (`self.Body`) (* (`self.SwingForce`) InputAxis) "None" false))

(fn `ToggleRagdoll`
  (params (IsOn :type Boolean))
  (locals (Ragdolling :type Boolean) (Thigh_l :type Name :default "Thigh_l") (Thigh_r :type Name :default "thigh_r") (Pelvis :type Name :default "pelvis"))
  (`SkeletalMeshComponent.SetAllBodiesBelowSimulatePhysics` (`self.Model`) (`self.RagdollBone`) IsOn false))

(fn `UpdatePlayer`
  ;[1 1 1] Modify player only after launch and when they haven't collided
  (if (and (`self.Launched`) (not (`self.Respawning`)))
    (`self.ApplyRotationToModel`)
    (`self.UpdateTrackedVariables`)
    (`self.IsAirborne`)
    (`self.CheckRequireRespawn`)))

(fn `UpdateTrackedVariables`
  ;[1 1 1] Re-evaluate variables that are pulled from Game Mode and send to HUD
  (set `self.Speed` (`KismetMathLibrary.VSize` (`SceneComponent.GetComponentVelocity` (`self.Body`)))))

(fn `UpDownMovement`
  (params (InputAxis :type "Float (double-precision)"))
  (if (!= InputAxis 0.0)
    (switch `/Game/Data/ENUM_PlayerState` (`self.CurrentState`)
      (:`NewEnumerator0`
        (`self.Swing` InputAxis))
      (:`NewEnumerator1`
        (`self.AdjustSpeed` InputAxis)))))

(fn `UserConstructionScript`)