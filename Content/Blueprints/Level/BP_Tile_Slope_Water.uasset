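; Water slope level tile that dresses itself with fences, trees, clouds and a log when constructed.
; The construction script builds fences from a reduced segment count, spawns the scenery, then pitches the whole actor by TileRot for the slope.
; SpawnLog adds a child actor at the transform of a randomly picked lane from the middle, first left and first right lanes.
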(fn `SpawnLog`
  (bind _output_get (set `self.LaneArray` (`|MakeArray` (`self.MiddleLane`) (`self.LeftLane1`) (`self.RightLane1`))))
  (`AddComponent|NODE_AddChildActorComponent-0` :`RelativeTransform` (`SceneComponent.GetRelativeTransform` (`/Game/Blueprints/BP_Macros.SelectRandomFromArray` _output_get))))

(fn `UserConstructionScript`
  (`self.ConstructFences` (- (`self.NumSegments`) 5))
  (`self.SpawnTrees` 5)
  (`self.SpawnClouds` 6)
  (`self.SpawnLog`)
  (`self.K2_SetActorRotation` (`KismetMathLibrary.MakeRotator` 0.0 (`self.TileRot`))))