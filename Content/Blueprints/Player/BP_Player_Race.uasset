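; Race variant of the player Blueprint that, on BeginPlay after the parent's logic, sets up helper visibility based on SwingingEnabled.
; SpawnHelpers only toggles visibility, hiding or showing Helpers and both P1 and P2 hand pairs, with hands set individually because propagation reaches one level.
; When swinging is disabled, the helpers are hidden and Launch is called.
; A separate custom event destroys the actor after a given delay.
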(event `self.ReceiveBeginPlay`
  (`parent.ReceiveBeginPlay`)
  (`self.SpawnHelpers`))

(event `CustomEvent`
  (params (DelayTime :type "Float (double-precision)"))
  (`KismetSystemLibrary.Delay` DelayTime)
  (`self.K2_DestroyActor`))

(fn `SpawnHelpers`
  (locals (HelpersSpawned :type Boolean))
  (bind _helpersspawned (`local.HelpersSpawned`))
  (`|ExecutionSequence`
    (:`then_0`
      ;[1 1 1] Inverted as toggling 'hidden' is used
      ; True = component hidden
      ; False = visible
      (set `local.HelpersSpawned` (not (`self.SwingingEnabled`)))
      ;[1 1 1] Hidden in game propagates only to children 1 level below, need to further hide children of children (Hands)
      (`SceneComponent.SetHiddenInGame` (`self.Helpers`) _helpersspawned true)
      (`SceneComponent.SetHiddenInGame` (`self.P1LeftHand`) _helpersspawned false)
      (`SceneComponent.SetHiddenInGame` (`self.P1RightHand`) _helpersspawned false)
      (`SceneComponent.SetHiddenInGame` (`self.P2LeftHand`) _helpersspawned false)
      (`SceneComponent.SetHiddenInGame` (`self.P2RightHand`) _helpersspawned false))
    (:`then_1`
      (if (not (`self.SwingingEnabled`))
        (`self.Launch`)))))

(fn `UserConstructionScript`
  (`parent.UserConstructionScript`))